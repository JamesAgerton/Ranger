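; Ranger component that manages a player's monster collection and a size-limited roster of battle monsters.
; New monsters join the collection and fill free roster slots, while removal clears them from both.
; SpawnFromRoster spawns only monsters with HP remaining.
; GetRosterCharacters spawns fresh hidden actors at the player pawn on every call, which GetRosterCombat uses to initialize and return combat components from roster stats.
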(fn GetRosterCharacters
  (bind _returnvalue (Game|Player|GetPlayerPawn 0))
  (bind _returnvalue_2 (Transformation|GetActorTransform _returnvalue))
  (Utilities|Array|Clear (LocalVariables|GetRosterCharacters))
  (for _array_element (Variables|Ranger|GetRoster)
    (bind _returnvalue_3 (Game|SpawnActorfromClass "/Game/Blueprints/Monsters/R_Base_Monster_BP.R_Base_Monster_BP_C" (Math|Transform|MakeTransform (+ (.location _returnvalue_2) "0, 0, 0") (.rotation _returnvalue_2) (.scale _returnvalue_2)) "Undefined" 0 _array_element 0))
    (Rendering|SetActorHiddenInGame _returnvalue_3 true)
    (Utilities|Array|Add (LocalVariables|GetRosterCharacters) _returnvalue_3))
  (return (LocalVariables|GetRosterCharacters)))

(fn AddtoCollection
  (params (NewMonster :type R%20Individual%20Struct%20Structure))
  (if (Utilities|Array|ContainsItem (Variables|Ranger|GetCollection) NewMonster)
    (Development|PrintString "Monster already exists in collection")
    (else
      (if (>= (Utilities|Array|Length (Variables|Ranger|GetRoster)) (Variables|Default|GetRosterSize))
        _
        (else
          (Utilities|Array|Add (Variables|Ranger|GetRoster) NewMonster)))
      (Utilities|Array|Add (Variables|Ranger|GetCollection) NewMonster))))

(fn RemovefromCollection
  (params (MonsterToRemove :type R%20Individual%20Struct%20Structure))
  ;[1 1 1] Check if the monster exists in your collection
  (if (Utilities|Array|ContainsItem (Variables|Ranger|GetCollection) MonsterToRemove)
    ;[1 1 1] Remove from your collection
    (bind _returnvalue (Utilities|Array|RemoveItem (Variables|Ranger|GetCollection) MonsterToRemove))
    (if _returnvalue
      (Development|PrintString "Removed from collection")
      ;[1 1 1] Check if it exists in your roster
      (if (Utilities|Array|ContainsItem (Variables|Ranger|GetRoster) MonsterToRemove)
        ;[1 1 1] Remove from Roster
        (bind _returnvalue_2 (Utilities|Array|RemoveItem (Variables|Ranger|GetRoster) MonsterToRemove))
        (if _returnvalue_2
          (Development|PrintString "Removed from your roster")
          (else
            (Development|PrintString "Failed to remove from your roster" true true "(R=1.000000,G=0.034294,B=0.000000,A=1.000000)")))
        (else
          (Development|PrintString "Does not exist in your roster")))
      (else
        (Development|PrintString "Failed to remove from collection" true true "(R=1.000000,G=0.059606,B=0.000000,A=1.000000)")))
    (else
      (Development|PrintString "Does not exist in your collection" true true "(R=1.000000,G=0.068094,B=0.000000,A=1.000000)"))))

(fn SpawnfromRoster
  (params (RosterIndex :type Integer) (Transform :type Transform))
  (bind _roster (Variables|Ranger|GetRoster))
  (bind _output (Utilities|Array|Get(acopy) _roster RosterIndex))
  (if (> (.hp_current (.Combat_Stats (Utilities|Struct|BreakR_Individual_Struct _output))) 0.0)
    (Game|SpawnActorfromClass "/Game/Blueprints/Monsters/R_Base_Monster_BP.R_Base_Monster_BP_C" Transform "AlwaysSpawn" 0 _output 0)
    (else
      (Development|PrintString "That monster cannot fight"))))

(fn GetRosterIndividuals
  (return (Variables|Ranger|GetRoster)))

(fn GetRosterCombat
  (bind _rostercharacters1 (CallFunction|GetRosterCharacters))
  (for (_array_element _array_index) _rostercharacters1
    (Default|SetData (Actor|GetComponentbyClass _array_element "/Game/Blueprints/Combat/R_CombatBase_C.R_CombatBase_C_C") (.Combat_Stats (Utilities|Struct|BreakR_Individual_Struct (Utilities|Array|Get(acopy) (Variables|Ranger|GetRoster) _array_index))) (.Stats (Utilities|Struct|BreakR_Individual_Struct (Utilities|Array|Get(acopy) (Variables|Ranger|GetRoster) _array_index))))
    (Utilities|Array|Add (LocalVariables|GetCombatComponents) (Actor|GetComponentbyClass _array_element "/Game/Blueprints/Combat/R_CombatBase_C.R_CombatBase_C_C")))
  (return (LocalVariables|GetCombatComponents)))