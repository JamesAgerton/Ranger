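; Capture actor that follows the player pawn and produces render targets for landscape deformation around it.
; A looping timer moves it in texel-snapped steps, captures the scene, and keeps its planes at the pawn's height.
; Each tick then draws persistent deformation, shifted by the move offset, plus blurred and normal targets through dynamic materials.
; Capture size and position go to a landscape material parameter collection.
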(event Custom|CaptureTimer
  (Utilities|FlowControl|Sequence
    (:then_0
      (CallFunction|MoveCapture)
      (Rendering|SceneCapture|CaptureScene (Variables|Default|GetSceneCapture) :!class /Script/Engine.SceneCaptureComponent2D))
    (:then_1
      (CallFunction|DrawLandscapeRTs))
    (:then_2
      (CallFunction|MovePlanes))))

(event EventBeginPlay
  (Utilities|FlowControl|Sequence
    (:then_0
      (Rendering|Material|SetScalarParameterValue "/Game/Materials/Landscape/Landscape_MPC.Landscape_MPC" "CaptureSize" (Variables|/Script/Engine.SceneCaptureComponent2D|GetOrthoWidth (Variables|Default|GetSceneCapture)) :!class /Script/Engine.KismetMaterialLibrary)
      (bind _returnvalue (Rendering|Material|CreateDynamicMaterialInstance "/Game/Materials/Landscape/Offset/DrawToDeformationPersistent_M.DrawToDeformationPersistent_M" "None" "None" :!class /Script/Engine.KismetMaterialLibrary))
      (Variables|Default|SetDrawMaterial _returnvalue)
      (bind _returnvalue_2 (Rendering|Material|CreateDynamicMaterialInstance "/Game/Materials/Landscape/Offset/BlurDeformation_M.BlurDeformation_M" "None" "None" :!class /Script/Engine.KismetMaterialLibrary))
      (Variables|Default|SetBlurMaterial _returnvalue_2)
      (bind _returnvalue_3 (Rendering|Material|CreateDynamicMaterialInstance "/Game/Materials/Landscape/Offset/DrawDeformationNormal_M_Inst.DrawDeformationNormal_M_Inst" "None" "None" :!class /Script/Engine.KismetMaterialLibrary))
      (Variables|Default|SetNormalMaterial _returnvalue_3))
    (:then_1
      (Rendering|ClearRenderTarget2D "/Game/Materials/Landscape/Offset/Deformation_RT.Deformation_RT")
      (Rendering|ClearRenderTarget2D "/Game/Materials/Landscape/Offset/DeformationPersistent_RT.DeformationPersistent_RT")
      (Rendering|ClearRenderTarget2D "/Game/Materials/Landscape/Offset/BlurredDeformation_RT.BlurredDeformation_RT")
      (Rendering|ClearRenderTarget2D "/Game/Materials/Landscape/Offset/DeformationNormal_RT.DeformationNormal_RT"))
    (:then_2
      (Utilities|Time|SetTimerbyFunctionName 0 "CaptureTimer" 0.032 true))))

(fn ConstructionScript)

(fn DrawLandscapeRTs
  (bind _moveoffset (Variables|Default|GetMoveOffset))
  (bind _scenecapture (Variables|Default|GetSceneCapture))
  (bind _orthowidth (Variables|/Script/Engine.SceneCaptureComponent2D|GetOrthoWidth _scenecapture))
  (Rendering|Material|SetVectorParameterValue (Variables|Default|GetDrawMaterial) "Offset" (Utilities|Struct|MakeLinearColor (/ (.x _moveoffset) _orthowidth) (/ (.y _moveoffset) _orthowidth) 0.0 1.0) :!class /Script/Engine.MaterialInstanceDynamic)
  (Rendering|DrawMaterialtoRenderTarget "/Game/Materials/Landscape/Offset/DeformationPersistent_RT.DeformationPersistent_RT" (Variables|Default|GetDrawMaterial))
  (Rendering|DrawMaterialtoRenderTarget "/Game/Materials/Landscape/Offset/BlurredDeformation_RT.BlurredDeformation_RT" (Variables|Default|GetBlurMaterial))
  (Rendering|DrawMaterialtoRenderTarget "/Game/Materials/Landscape/Offset/DeformationNormal_RT.DeformationNormal_RT" (Variables|Default|GetNormalMaterial)))

(fn MoveCapture
  (bind _returnvalue (Transformation|GetActorLocation))
  (bind _returnvalue_2 (Transformation|GetActorLocation))
  (bind _returnvalue_3 (/ 1.0 2048.0))
  (bind _scenecapture (Variables|Default|GetSceneCapture))
  (bind _playerpawn (Variables|Default|GetPlayerPawn))
  (bind _returnvalue_4 (Transformation|GetActorLocation _playerpawn))
  (bind _orthowidth (Variables|/Script/Engine.SceneCaptureComponent2D|GetOrthoWidth _scenecapture))
  (bind _returnvalue_5 (* _orthowidth _returnvalue_3))
  (bind _returnvalue_6 (/ (.y _returnvalue_4) _returnvalue_5))
  (bind _returnvalue_7 (/ (.x _returnvalue_4) _returnvalue_5))
  (bind _returnvalue_8 (+ _returnvalue_6 0.5))
  (bind _returnvalue_9 (+ _returnvalue_7 0.5))
  (bind _returnvalue_10 (Math|Float|Floor _returnvalue_8))
  (bind _returnvalue_11 (Math|Float|Floor _returnvalue_9))
  (bind _returnvalue_12 (* _returnvalue_10 _returnvalue_5))
  (bind _returnvalue_13 (* _returnvalue_11 _returnvalue_5))
  (bind _returnvalue_14 (Math|Vector|MakeVector _returnvalue_13 _returnvalue_12 0.0))
  (bind _returnvalue_15 (- _returnvalue_14 _returnvalue_2))
  (bind _output_get (Variables|Default|SetMoveOffset (Math|Vector2D|MakeVector2D (.x _returnvalue_15) (.y _returnvalue_15))))
  (Transformation|AddActorWorldOffset (Math|Vector|MakeVector (.x _output_get) (.y _output_get) 0.0))
  (Rendering|Material|SetVectorParameterValue "/Game/Materials/Landscape/Landscape_MPC.Landscape_MPC" "OffsetPosition" (Utilities|Struct|MakeLinearColor (.x _returnvalue) (.y _returnvalue) 0.0 0.0) :!class /Script/Engine.KismetMaterialLibrary))

(fn MovePlanes
  (Transformation|SetRelativeLocation (Variables|Default|GetPlanes) (Math|Vector|MakeVector 0.0 0.0 (- (.z (Transformation|GetActorLocation (Variables|Default|GetPlayerPawn))) (.z (Transformation|GetActorLocation)))) false false))

(fn SetPlayerPawn
  (params (PlayerPawn :type Actor%20Object%20Reference))
  (Variables|Default|SetPlayerPawn PlayerPawn))