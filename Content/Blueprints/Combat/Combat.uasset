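; Combat Blueprint that initializes a combatant's stats and action point pool.
; SetStats stores the incoming stats, sets current HP from the truncated HP stat, and derives both current and maximum action points from Speed.
; The action point count comes from sampling a float curve at the Speed value and truncating it, so the speed-to-AP relationship is shaped by curve data.
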(fn SetStats
  (params (Stats :type Stat%20Struct%20Structure))
  (Variables|Default|SetStats Stats)
  (Variables|Default|SetCurrentHP (Math|Float|Truncate (.hp (Variables|Default|GetStats))))
  (bind _output_get (Variables|Default|SetActionPoints (CallFunction|APCalculation (.speed (Variables|Default|GetStats)))))
  (Variables|Default|SetActionPointMax _output_get))

(fn APCalculation
  (params (Speed :type Float%20%28double-precision%29))
  (return (Math|Float|Truncate (Math|Curves|GetFloatValue (Variables|Default|GetAP_Curve) Speed))))