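; Combat manager Blueprint that sets up turn order for a fight between allied and enemy parties.
; StartCombat_Party_SERVER clears and stores both parties, builds the combatant order, then prints all three lists with Speed for debugging.
; InitiateCombatantOrder attempts a descending-Speed insertion, but compares allies' Stamina and also appends combatants after inserting them.
; SetPhase and SelectNextCombatant are empty stubs, and Tick only returns false.
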(event Custom|StartCombat_Party_SERVER
  (params (Allies :type Array%20of%20R%20Combat%20Base%20C%20Object%20References) (Enemies :type Array%20of%20R%20Combat%20Base%20C%20Object%20References))
  (CallFunction|ClearParties)
  (Development|PrintString "Start Combat")
  (Utilities|FlowControl|Sequence
    (:then_0
      ;[1 1 1] Add parties to combat order
      (Variables|Default|SetAlliedParty_Comps Allies)
      (Variables|Default|SetEnemyParty_Comps Enemies)
      (CallFunction|InitiateCombatantOrder)
      (Utilities|FlowControl|Sequence
        (:then_0
          (Development|PrintString "||||||||||||||||||||||||||||||||||||||||||||||||||||||||||| -- Allies:")
          (for _array_element (Variables|Default|GetAlliedParty_Comps)
            (Development|PrintString (Utilities|String|Append (Utilities|GetDisplayName _array_element) ": SPEED:" (Utilities|String|ToString(Integer) (.Speed (Utilities|Struct|BreakR_Stat_Struct (Variables|/Game/Blueprints/Combat/R_CombatBase_C.R_CombatBase_C_C|GetStats _array_element))))))))
        (:then_1
          (Development|PrintString "||||||||||||||||||||||||||||||||||||||||||||||||||||||||||| -- Enemies:")
          (for _array_element_2 (Variables|Default|GetEnemyParty_Comps)
            (Development|PrintString (Utilities|String|Append (Utilities|GetDisplayName _array_element_2) ": SPEED:" (Utilities|String|ToString(Integer) (.Speed (Utilities|Struct|BreakR_Stat_Struct (Variables|/Game/Blueprints/Combat/R_CombatBase_C.R_CombatBase_C_C|GetStats _array_element_2))))))))
        (:then_2
          (Development|PrintString "||||||||||||||||||||||||||||||||||||||||||||||||||||||||||| -- COMBATANT ORDER:")
          (for _array_element_3 (Variables|Default|GetCombatantOrder_Comps)
            (Development|PrintString (Utilities|String|Append (Utilities|GetDisplayName _array_element_3) ": SPEED:" (Utilities|String|ToString(Integer) (.Speed (Utilities|Struct|BreakR_Stat_Struct (Variables|/Game/Blueprints/Combat/R_CombatBase_C.R_CombatBase_C_C|GetStats _array_element_3))))))))))))

(fn Tick
  (params (DeltaSeconds :type Float%20%28double-precision%29))
  (return false))

(fn SetPhase
  (params (Phase :type R_CombatPhase%20Enum :default "NewEnumerator0")))

(fn SelectNextCombatant)

(fn ClearParties
  (Utilities|Array|Clear (Variables|Default|GetCombatantOrder_Comps))
  (Utilities|Array|Clear (Variables|Default|GetAlliedParty_Comps))
  (Utilities|Array|Clear (Variables|Default|GetEnemyParty_Comps)))

(fn InitiateCombatantOrder
  (bind _combatantorder_comps (Variables|Default|GetCombatantOrder_Comps))
  (bind _returnvalue (Utilities|Array|Length _combatantorder_comps))
  (bind _returnvalue_2 (> _returnvalue 0))
  (for _array_element (Variables|Default|GetAlliedParty_Comps)
    (if (and (> (Utilities|Array|Length (Variables|Default|GetAlliedParty_Comps)) 0) _returnvalue_2)
      (bind (_array_element_2 _array_index) (Utilities|Array|ForEachLoopwithBreak (Variables|Default|GetCombatantOrder_Comps) :!label _label)
        (:LoopBody
          (if (< (.speed (Variables|/Game/Blueprints/Combat/R_CombatBase_C.R_CombatBase_C_C|GetStats _array_element_2)) (.stamina (Variables|/Game/Blueprints/Combat/R_CombatBase_C.R_CombatBase_C_C|GetStats _array_element)))
            (Utilities|Array|Insert (Variables|Default|GetCombatantOrder_Comps) _array_element _array_index)
            (goto _label Break)))
        (:Completed
          (Utilities|Array|Add (Variables|Default|GetCombatantOrder_Comps) _array_element :!label _label_2)))
      (else
        (goto _label_2))))
  (for _array_element_3 (Variables|Default|GetEnemyParty_Comps)
    (if (and (> (Utilities|Array|Length (Variables|Default|GetEnemyParty_Comps)) 0) _returnvalue_2)
      (bind (_array_element_4 _array_index_2) (Utilities|Array|ForEachLoopwithBreak (Variables|Default|GetCombatantOrder_Comps) :!label _label_3)
        (:LoopBody
          (if (< (.speed (Variables|/Game/Blueprints/Combat/R_CombatBase_C.R_CombatBase_C_C|GetStats _array_element_4)) (.speed (Variables|/Game/Blueprints/Combat/R_CombatBase_C.R_CombatBase_C_C|GetStats _array_element_3)))
            (Utilities|Array|Insert (Variables|Default|GetCombatantOrder_Comps) _array_element_3 _array_index_2)
            (goto _label_3 Break)))
        (:Completed
          (Utilities|Array|Add (Variables|Default|GetCombatantOrder_Comps) _array_element_3 :!label _label_4)))
      (else
        (goto _label_4)))))