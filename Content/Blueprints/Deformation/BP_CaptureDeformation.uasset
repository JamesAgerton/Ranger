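; Actor that records landscape deformation around the player into render targets.
; A looping timer moves it to the player's XY, snapped to texel-sized steps of the ortho width, then runs a scene capture.
; It publishes its position to MPC_Landscape and passes the move offset to the persistent draw material.
; Dynamic materials then draw the persistent, blurred and normal deformation render targets, which are cleared at BeginPlay.
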(event Custom|CaptureTimer
  (Utilities|FlowControl|Sequence
    (:then_0
      (CallFunction|MoveCapture)
      (Rendering|SceneCapture|CaptureScene (Variables|Default|GetSceneCaptureComponent2D) :!class /Script/Engine.SceneCaptureComponent2D))
    (:then_1
      (CallFunction|DrawtoRTs))))

(event EventBeginPlay
  (Utilities|FlowControl|Sequence
    (:then_0
      ;[1 1 1] Setup default variables
      (Variables|Default|SetPlayerPawn (Game|GetPlayerCharacter 0))
      (Rendering|Material|SetScalarParameterValue "/Game/Materials/Landscape/MPC_Landscape.MPC_Landscape" "CaptureSize" (Variables|/Script/Engine.SceneCaptureComponent2D|GetOrthoWidth (Variables|Default|GetSceneCaptureComponent2D)) :!class /Script/Engine.KismetMaterialLibrary))
    (:then_1
      ;[1 1 1] Setup Dynamic Materials
      (bind _returnvalue (Rendering|Material|CreateDynamicMaterialInstance "/Game/Materials/Landscape/Offset/M_DrawToDeformationPersistent.M_DrawToDeformationPersistent" "None" "None" :!class /Script/Engine.KismetMaterialLibrary))
      (Variables|Default|SetDrawPersistent _returnvalue)
      (bind _returnvalue_2 (Rendering|Material|CreateDynamicMaterialInstance "/Game/Materials/Landscape/Offset/M_DrawToDeformationBlurred.M_DrawToDeformationBlurred" "None" "None" :!class /Script/Engine.KismetMaterialLibrary))
      (Variables|Default|SetDrawBlurred _returnvalue_2)
      (bind _returnvalue_3 (Rendering|Material|CreateDynamicMaterialInstance "/Game/Materials/Landscape/Offset/M_DrawToDeformationNormal_Inst.M_DrawToDeformationNormal_Inst" "None" "None" :!class /Script/Engine.KismetMaterialLibrary))
      (Variables|Default|SetDrawNormal _returnvalue_3))
    (:then_2
      ;[1 1 1] Clear RenderTargets
      (Rendering|ClearRenderTarget2D "/Game/Materials/Landscape/Offset/RT_Capture.RT_Capture" "(R=0.000000,G=0.000000,B=0.000000,A=0.000000)")
      (Rendering|ClearRenderTarget2D "/Game/Materials/Landscape/Offset/RT_DeformationPersistent.RT_DeformationPersistent" "(R=0.000000,G=0.000000,B=0.000000,A=0.000000)")
      (Rendering|ClearRenderTarget2D "/Game/Materials/Landscape/Offset/RT_DeformationBlurred.RT_DeformationBlurred" "(R=0.000000,G=0.000000,B=0.000000,A=0.000000)")
      (Rendering|ClearRenderTarget2D "/Game/Materials/Landscape/Offset/RT_DeformationNormal.RT_DeformationNormal" "(R=0.000000,G=0.000000,B=0.000000,A=0.000000)"))
    (:then_3
      ;[1 1 1] Start the capture timer
      (Utilities|Time|SetTimerbyFunctionName self "CaptureTimer" 0.032 true))))

(fn ConstructionScript)

(fn MoveCapture
  (bind _returnvalue (Transformation|GetActorLocation))
  (bind _returnvalue_2 (Transformation|GetActorLocation))
  (bind _returnvalue_3 (/ 1.0 2048.0))
  (bind _playerpawn (Variables|Default|GetPlayerPawn))
  (bind _scenecapturecomponent2d (Variables|Default|GetSceneCaptureComponent2D))
  (bind _scenecapturecomponent2d_2 (Variables|Default|GetSceneCaptureComponent2D))
  (bind _returnvalue_4 (Transformation|GetActorLocation _playerpawn))
  (bind _orthowidth (Variables|/Script/Engine.SceneCaptureComponent2D|GetOrthoWidth _scenecapturecomponent2d_2))
  (bind _orthowidth_2 (Variables|/Script/Engine.SceneCaptureComponent2D|GetOrthoWidth _scenecapturecomponent2d))
  (bind _returnvalue_5 (* _orthowidth_2 _returnvalue_3))
  (bind _returnvalue_6 (/ (.x _returnvalue_4) _returnvalue_5))
  (bind _returnvalue_7 (/ (.y _returnvalue_4) _returnvalue_5))
  (bind _returnvalue_8 (+ _returnvalue_6 0.5))
  (bind _returnvalue_9 (+ _returnvalue_7 0.5))
  (bind _returnvalue_10 (Math|Float|Floor _returnvalue_9))
  (bind _returnvalue_11 (Math|Float|Floor _returnvalue_8))
  (bind _returnvalue_12 (* _returnvalue_10 _returnvalue_5))
  (bind _returnvalue_13 (* _returnvalue_11 _returnvalue_5))
  (bind _returnvalue_14 (Math|Vector|MakeVector _returnvalue_13 _returnvalue_12 0.0))
  (bind _returnvalue_15 (- _returnvalue_14 _returnvalue))
  (bind _output_get (Variables|Default|SetMoveOffset (Math|Vector2D|MakeVector2D (.x _returnvalue_15) (.y _returnvalue_15))))
  (Transformation|AddActorWorldOffset (Math|Vector|MakeVector (.x _output_get) (.y _output_get) 0.0))
  ;[1 1 1] Set parameter collection
  (Rendering|Material|SetVectorParameterValue "/Game/Materials/Landscape/MPC_Landscape.MPC_Landscape" "OffsetPosition" (Utilities|Struct|MakeLinearColor (.x _returnvalue_2) (.y _returnvalue_2) 0.0 1.0) :!class /Script/Engine.KismetMaterialLibrary)
  ;[1 1 1] Set offset in draw persistent material
  (Rendering|Material|SetVectorParameterValue (Variables|Default|GetDrawPersistent) "Offset" (Utilities|Struct|MakeLinearColor (/ (.x (Variables|Default|GetMoveOffset)) _orthowidth) (/ (.y (Variables|Default|GetMoveOffset)) _orthowidth) 0.0 1.0) :!class /Script/Engine.MaterialInstanceDynamic))

(fn DrawtoRTs
  (Rendering|DrawMaterialtoRenderTarget "/Game/Materials/Landscape/Offset/RT_DeformationPersistent.RT_DeformationPersistent" (Variables|Default|GetDrawPersistent))
  (Rendering|DrawMaterialtoRenderTarget "/Game/Materials/Landscape/Offset/RT_DeformationBlurred.RT_DeformationBlurred" (Variables|Default|GetDrawBlurred))
  (Rendering|DrawMaterialtoRenderTarget "/Game/Materials/Landscape/Offset/RT_DeformationNormal.RT_DeformationNormal" (Variables|Default|GetDrawNormal)))