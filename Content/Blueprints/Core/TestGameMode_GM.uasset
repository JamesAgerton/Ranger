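; TestGameMode_GM is a test game mode that reveals player name tags in the world.
; On BeginPlay and on every PostLogin it waits three seconds, then gathers all R_Base_Character_BP actors.
; For each, it casts the NameTag widget to WB_Username, calls ClientShowName and prints a debug message.
; A branch meant to hide the local player's own tag is left disconnected.
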(event EventBeginPlay
  (Utilities|FlowControl|Delay 3.0)
  (bind _outactors (Actor|GetAllActorsOfClass "/Game/Blueprints/Character/R_Base_Character_BP.R_Base_Character_BP_C"))
  (for _array_element _outactors
    (bind _aswb_username (Utilities|Casting|CastToWB_Username (UserInterface|GetUserWidgetObject (Variables|/Game/Blueprints/Character/R_Base_Character_BP.R_Base_Character_BP_C|GetNameTag _array_element))))
    (Default|ClientShowName _aswb_username)
    (Development|PrintString "Shown")))

(event EventPostLogin
  (params (NewPlayer :type Player%20Controller%20Object%20Reference))
  (Utilities|FlowControl|Delay 3.0)
  (bind _outactors (Actor|GetAllActorsOfClass "/Game/Blueprints/Character/R_Base_Character_BP.R_Base_Character_BP_C"))
  (for _array_element _outactors
    (bind _aswb_username (Utilities|Casting|CastToWB_Username (UserInterface|GetUserWidgetObject (Variables|/Game/Blueprints/Character/R_Base_Character_BP.R_Base_Character_BP_C|GetNameTag _array_element))))
    (Default|ClientShowName _aswb_username)
    (Development|PrintString "Shown")))

(fn ConstructionScript)