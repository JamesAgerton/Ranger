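; Game state Blueprint that tracks the in-game time of day and calendar date, starting from a fixed date.
; A looping timer advances a wrapped 0–1 day fraction, scaled by the game mode's day length.
; Wrapping calls DateForward, which as written changes the date only on day 30, rolling into the next month or year.
; UpdateTime overrides the time, and getters expose time and date.
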(event EventBeginPlay
  (bind _asr_gm_framework (Utilities|Casting|CastToR_GM_Framework (Game|GetGameMode)))
  (Variables|Ref|SetGameMode _asr_gm_framework)
  (Variables|Time|SetSystemDate (Math|DateTime|MakeDateTime 112 6 19))
  (Utilities|Time|SetTimerbyFunctionName 0 "ProgressTime" (Variables|Default|GetTimeLoopDeltaS) true 0.2))

(event EventUpdateTime
  (params (TimePercent :type Float%20%28double-precision%29))
  (Variables|Time|SetTimeOfDayPercent TimePercent))

(fn ConstructionScript)

(fn ProgressTime
  (if (> (+ (/ (/ (Variables|Default|GetTimeLoopDeltaS) 6e+01) (Variables|/Game/Blueprints/Core/R_GM_Framework.R_GM_Framework_C|GetLengthOfDayInMinutes (Variables|Ref|GetGameMode))) (Variables|Time|GetTimeOfDayPercent)) 1.0)
    (CallFunction|DateForward))
  (Variables|Time|SetTimeOfDayPercent (Class|KismetMathLibrary|FWrap (+ (/ (/ (Variables|Default|GetTimeLoopDeltaS) 6e+01) (Variables|/Game/Blueprints/Core/R_GM_Framework.R_GM_Framework_C|GetLengthOfDayInMinutes (Variables|Ref|GetGameMode))) (Variables|Time|GetTimeOfDayPercent)) 0.0 1.0)))

(fn DateForward
  (Utilities|FlowControl|Sequence
    (:then_0
      (LocalVariables|SetYear (.year (Variables|Time|GetSystemDate)))
      (LocalVariables|SetMonth (.month (Variables|Time|GetSystemDate)))
      (LocalVariables|SetDay (.day (Variables|Time|GetSystemDate))))
    (:then_1
      (if (== (LocalVariables|GetDay) 30)
        (bind _result (Math|Integer|IncrementInt (LocalVariables|GetDay))
          (:%20%20
            (if (> _result 30)
              (LocalVariables|SetDay 1)
              (bind _result_2 (Math|Integer|IncrementInt (LocalVariables|GetMonth))
                (:%20%20
                  (if (> _result_2 12)
                    (LocalVariables|SetMonth 1)
                    (Math|Integer|IncrementInt (LocalVariables|GetYear))))))))))
    (:then_2
      (Variables|Time|SetSystemDate (Math|DateTime|MakeDateTime (LocalVariables|GetYear) (LocalVariables|GetMonth) (LocalVariables|GetDay) 0 0 0 0)))))

(fn GetSystemDate
  (return (Variables|Time|GetSystemDate)))

(fn GetTime
  (return (Variables|Time|GetTimeOfDayPercent)))