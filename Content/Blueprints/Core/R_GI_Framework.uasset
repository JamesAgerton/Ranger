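; Game instance Blueprint that manages the player's save data and destroys the session on network errors or on request.
; LoadGame reads the slot into SaveGameData or calls NewSave, which clears any existing slot and creates player info with random trainer and secret IDs in memory.
; LoadPlayerData restores the character's saved location.
; A looping autosave timer calls Save_PlayerData, but its location capture and async slot write are disconnected, so nothing is saved.
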(event Custom|DestroySession
  ;[1 1 1] Network error  / end session
  (|DestroySession (Game|GetPlayerController 0)
    (:OnSuccess
      (Development|PrintString "Session destroyed successfully"))
    (:OnFailure
      (Development|PrintString "Session could not be destroyed"))))

(event Custom|Save_PlayerData
  (bind _asr_base_character_bp (Utilities|Casting|CastToR_Base_Character_BP (Game|GetPlayerCharacter 0)))
  (Variables|Default|SetPlayerRef _asr_base_character_bp)
  (bind _returnvalue (SaveGame|DoesSaveGameExist (Variables|Default|GetSaveSlotName)))
  (if (not _returnvalue)
    (Development|PrintString "No SaveData in slot to autosave to")))

(event Custom|Load%20Game
  (bind _returnvalue (SaveGame|DoesSaveGameExist (Variables|Default|GetSaveSlotName)))
  (if _returnvalue
    (bind _returnvalue_2 (SaveGame|LoadGamefromSlot (Variables|Default|GetSaveSlotName)))
    (bind _asr_save_game_object (Utilities|Casting|CastToR_SaveGameObject _returnvalue_2))
    (Variables|Default|SetSaveGameData _asr_save_game_object)
    (else
      (bind _returnvalue_3 (SaveGame|CreateSaveGameObject "/Game/Blueprints/Core/SaveGame/R_SaveGameObject.R_SaveGameObject_C"))
      (Variables|Default|SetSaveGameData _returnvalue_3)
      (CallFunction|NewSave))))

(event Custom|StartAutoSave
  (Utilities|Time|SetTimerbyFunctionName self "Save_PlayerData" 5.0 true))

(event EventHandleNetworkError
  (params (FailureType :type ENetworkFailure%20Enum :default "NetDriverAlreadyExists") (bIsServer :type Boolean))
  ;[1 1 1] Network error  / end session
  (Development|PrintString (Utilities|String|EnumtoString FailureType))
  (|DestroySession (Game|GetPlayerController 0)
    (:OnSuccess
      (Development|PrintString "Session destroyed successfully"))
    (:OnFailure
      (Development|PrintString "Session could not be destroyed"))))

(fn LoadPlayerData
  (bind _asr_base_character_bp (Utilities|Casting|CastToR_Base_Character_BP (Game|GetPlayerCharacter 0))
    (:then
      (LocalVariables|SetPlayerRef _asr_base_character_bp)
      (bind _savegamedata (Variables|Default|GetSaveGameData)
        (:then
          (Transformation|SetActorLocation (LocalVariables|GetPlayerRef) (Default|GetPlayerLocation _savegamedata) false false))
        (:else
          (Development|PrintString "Savegamedata not valid"))))
    (:CastFailed
      (Development|PrintString "Could not cast character to R_BaseCharacter_BP"))))

(fn GetPlayerInfo
  (bind _returnvalue (SaveGame|DoesSaveGameExist (Variables|Default|GetSaveSlotName)))
  (if _returnvalue
    (CallFunction|LoadGame)
    (return (Default|GetPlayerInfo (Variables|Default|GetSaveGameData)))
    (else
      (Development|PrintString "Default Save Game doesn't exist"))))

(fn NewSave
  (bind _saveslotname (Variables|Default|GetSaveSlotName))
  (bind _returnvalue (SaveGame|DoesSaveGameExist _saveslotname))
  (if _returnvalue
    (SaveGame|DeleteGameinSlot _saveslotname))
  (bind _returnvalue_2 (SaveGame|CreateSaveGameObject "/Game/Blueprints/Core/SaveGame/R_SaveGameObject.R_SaveGameObject_C"))
  (Variables|Default|SetSaveGameData _returnvalue_2)
  (Default|SetPlayerInfo (Variables|Default|GetSaveGameData) (Utilities|Struct|MakePlayerData_Struct (Variables|Default|GetNameText) (Math|Random|RandomInteger 2147483647) (Math|Random|RandomInteger 2147483647) "NewEnumerator2")))