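; Sky actor that places the sun and other planets or moons as seen from a latitude and longitude on a tilted, rotating planet.
; Each tick, game-state day and orbit percentages drive a surface-frame matrix and orbital positions.
; The matrix's inverse rotates the sun light and maps spawned sphere meshes into local sky, with delta-time smoothing.
; IsMoon makes the first body the orbital parent; ShowDebug draws a scaled system diagram.
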(event EventBeginPlay
  (CallFunction|BeginPlay))

(event EventTick
  (params (DeltaSeconds :type Float%20%28single-precision%29))
  (CallFunction|MainFunction))

(fn ConstructionScript
  (Rendering|Debug|FlushPersistentDebugLines)
  (Class|KismetSystemLibrary|FlushDebugStrings)
  (CallFunction|CalculateMyPlanet false)
  (CallFunction|CalculateMatrix)
  (CallFunction|MoveSun)
  (CallFunction|CalculateMoons)
  (if (!= (Utilities|Array|Length (Variables|OrbitalComponents|Getmoons)) (Utilities|Array|Length (Variables|OrbitalComponents|GetOtherPlanets)))
    (CallFunction|MakeMoons))
  (for (_array_element _array_index) (Variables|OrbitalComponents|Getmoons)
    (Transformation|SetWorldTransform _array_element (Utilities|Array|Get(acopy) (Variables|OrbitalComponents|GetOtherPlanets_Dir) _array_index) false true))
  (CallFunction|DrawDebugDiagram))

(fn BeginPlay
  (bind _asr_gs_framework (Utilities|Casting|CastToR_GS_Framework (Game|GetGameState)))
  (Variables|Ref|SetGameState _asr_gs_framework))

(fn DrawDebugDiagram
  (if (Variables|Config|GetShowDebug)
    (LocalVariables|SetDiagramLocation (+ (Transformation|GetActorLocation) (Variables|Config|GetDebug_LocationOffset)))
    (Utilities|FlowControl|Sequence
      (:then_0
        (|DrawArrowsFromCenter))
      (:then_1
        (|DebugPlanet))
      (:then_2
        (|DrawSunPosition))
      (:then_3
        (|DrawMoons))
      (:then_4
        (|DrawSystemClock)))))

(fn CalculateMyPlanet
  (params (GetTimeDayPercent :type Boolean))
  (if GetTimeDayPercent
    (CallFunction|GetTimeDayPercent))
  (Utilities|FlowControl|Sequence
    (:then_0
      (Variables|OrbitalComponents|SetMy_UpDir (Math|Vector|Normalize (Math|Vector|RotateVectorAroundAxis (Math|Vector|CrossProduct (Math|Vector|RotateVectorAroundAxis (Math|Vector|MakeVector 1.0 0.0 0.0) (Variables|OrbitalComponents|GetMy_Inclination) "1.000000,0.000000,0.000000") (Math|Vector|RotateVectorAroundAxis (Math|Vector|MakeVector 0.0 1.0 0.0) (Variables|OrbitalComponents|GetMy_Inclination) "1.000000,0.000000,0.000000")) (Variables|OrbitalComponents|GetMy_InclArg) "0.000000,0.000000,1.000000")))
      (Variables|OrbitalComponents|SetMy_RightDir (Math|Vector|Normalize (Math|Vector|CrossProduct (Math|Vector|RotateVectorAroundAxis (Math|Vector|MakeVector 0.0 1.0 0.0) (* (Variables|Ref|GetTimePercent) -3.6e+02) (Variables|OrbitalComponents|GetMy_UpDir)) (Variables|OrbitalComponents|GetMy_UpDir))))
      (Variables|OrbitalComponents|SetMy_ForwardDir (Math|Vector|Normalize (Math|Vector|CrossProduct (Variables|OrbitalComponents|GetMy_UpDir) (Variables|OrbitalComponents|GetMy_RightDir)))))
    (:then_1
      (Variables|OrbitalComponents|SetMy_SurfaceUp (Math|Vector|Normalize (Math|Vector|RotateVectorAroundAxis (Math|Vector|RotateVectorAroundAxis (Variables|OrbitalComponents|GetMy_ForwardDir) (Variables|OrbitalComponents|GetMy_Latitude) (Variables|OrbitalComponents|GetMy_RightDir)) (Class|KismetMathLibrary|FWrap (Variables|OrbitalComponents|GetMy_Longitude) -1.8e+02 1.8e+02) (Variables|OrbitalComponents|GetMy_UpDir))))
      (Variables|OrbitalComponents|SetMy_SurfaceEast (Math|Vector|Normalize (Math|Vector|CrossProduct (Variables|OrbitalComponents|GetMy_SurfaceUp) (Variables|OrbitalComponents|GetMy_UpDir))))
      (Variables|OrbitalComponents|SetMy_SurfaceNorth (Math|Vector|Normalize (Math|Vector|CrossProduct (Variables|OrbitalComponents|GetMy_SurfaceEast) (Variables|OrbitalComponents|GetMy_SurfaceUp)))))))

(fn CalculateMoons
  (bind _otherplanets_dir (Variables|OrbitalComponents|GetOtherPlanets_Dir))
  (if (!= (Utilities|Array|Length (Variables|OrbitalComponents|GetOtherPlanets)) 0)
    (for (_array_element _array_index) (Variables|OrbitalComponents|GetOtherPlanets)
      (bind _orbit_percent (Class|BPITime|GetOrbitPercent(Message) (Variables|Ref|GetGameState) (.Orbital_Period (Utilities|Struct|BreakS_OrbitalData _array_element))))
      (LocalVariables|SetOrbitPercent _orbit_percent)
      (Utilities|Array|SetArrayElem (Variables|OrbitalComponents|GetOtherPlanets_Dir) _array_index (Math|Transform|MakeTransform (+ (* (Math|Vector|Normalize (Math|Vector|RotateVectorAroundAxis (Math|Vector|RotateVectorAroundAxis (Math|Vector|MakeVector (Math|Trig|Cos(Degrees) (+ (* (LocalVariables|GetOrbitPercent) -3.6e+02) (* (.Orbital_Argument (Utilities|Struct|BreakS_OrbitalData _array_element)) -1.0))) (Math|Trig|Sin(Degrees) (+ (* (LocalVariables|GetOrbitPercent) -3.6e+02) (* (.Orbital_Argument (Utilities|Struct|BreakS_OrbitalData _array_element)) -1.0))) 0.0) (.Orbital_Inclination (Utilities|Struct|BreakS_OrbitalData _array_element)) "1.000000,0.000000,0.000000") (.Orbital_IncArg (Utilities|Struct|BreakS_OrbitalData _array_element)) "0.000000,0.000000,1.000000")) (* (.Orbital_Radius (Utilities|Struct|BreakS_OrbitalData _array_element)) 1e+02 1e+03)) (Math|Vector|SelectVector (.location (Utilities|Array|Get(acopy) _otherplanets_dir)) "0, 0, 0" (Math|Boolean|ANDBoolean (Variables|OrbitalComponents|GetIsMoon) (!= _array_index 0) (!= (Utilities|Array|Length _otherplanets_dir) 0)))) "0, 0, 0" (|SetPlanetScale _array_element)) true))))

(fn MakeMoons
  (bind _moons (Variables|OrbitalComponents|Getmoons))
  (for _array_element _moons
    (Components|DestroyComponent _array_element))
  (Utilities|Array|Clear _moons)
  (for _array_element_2 (Variables|OrbitalComponents|GetOtherPlanets_Dir)
    (bind _returnvalue (AddComponent|AddStaticMeshComponent false _array_element_2))
    (bind _returnvalue_2 (Utilities|Array|Add (Variables|OrbitalComponents|Getmoons) _returnvalue))
    (Components|StaticMesh|SetStaticMesh _returnvalue "/Engine/ArtTools/RenderToTexture/Meshes/S_1_Unit_Sphere_HI.S_1_Unit_Sphere_HI")
    (Rendering|Components|SetLightingChannels _returnvalue false false true)
    (Variables|/Script/Engine.PrimitiveComponent|SetbEnableAutoLODGeneration _returnvalue false)
    (Collision|SetCollisionEnabled _returnvalue "NoCollision")
    (Rendering|Material|SetMaterial _returnvalue 0 (select (and (Variables|OrbitalComponents|GetIsMoon) (== _returnvalue_2 0)) "/Game/Materials/Sky/Moon_M_Inst.Moon_M_Inst" "/Game/Materials/Sky/Moon_M_Inst1.Moon_M_Inst1"))))

(fn CalculateMatrix
  (bind _my_surfaceup (Variables|OrbitalComponents|GetMy_SurfaceUp))
  (bind _my_surfaceeast (Variables|OrbitalComponents|GetMy_SurfaceEast))
  (bind _my_surfacenorth (Variables|OrbitalComponents|GetMy_SurfaceNorth))
  (bind _returnvalue (* _my_surfacenorth -1.0))
  (Variables|OrbitalComponents|SetMatrix (Utilities|Struct|MakeMatrix (Utilities|Struct|MakePlane 0.0 (.x _my_surfaceeast) (.y _my_surfaceeast) (.z _my_surfaceeast)) (Utilities|Struct|MakePlane 0.0 (.x _returnvalue) (.y _returnvalue) (.z _returnvalue)) (Utilities|Struct|MakePlane 0.0 (.x _my_surfaceup) (.y _my_surfaceup) (.z _my_surfaceup)) (Utilities|Struct|MakePlane 1.0 0.0 0.0 0.0))))

(fn MoveSun
  (bind _returnvalue (Math|Float|MakeLiteralFloat 6371.0))
  (bind _returnvalue_2 (* _returnvalue 1e+02 1e+03))
  (bind _returnvalue_3 (Math|Vector|MakeVector _returnvalue_2 0.0 0.0))
  (bind _returnvalue_4 (Math|Vector|Normalize _returnvalue_3))
  (bind _returnvalue_5 (Math|Vector|CrossProduct _returnvalue_4 "0.000000,0.000000,1.000000"))
  (bind _returnvalue_6 (Math|Vector|Normalize _returnvalue_5))
  (Variables|OrbitalComponents|SetSunDir _returnvalue_4)
  (Transformation|SetRelativeRotation (Variables|Default|GetSun_Light) (Math|Rotator|MakeRotationfromAxes (Math|Vector|Normalize (Class|KismetMathLibrary|MatrixInverseTransformVector (Variables|OrbitalComponents|GetMatrix) (Variables|OrbitalComponents|GetSunDir))) (Math|Vector|Normalize (Class|KismetMathLibrary|MatrixInverseTransformVector (Variables|OrbitalComponents|GetMatrix) _returnvalue_6)) (Math|Vector|Normalize (Class|KismetMathLibrary|MatrixInverseTransformVector (Variables|OrbitalComponents|GetMatrix) (Math|Vector|Normalize (Math|Vector|CrossProduct _returnvalue_4 _returnvalue_6))))) false false))

(fn GetTimeDayPercent
  (bind _daypercent (Class|BPITime|GetDayPercent(Message) (Variables|Ref|GetGameState)))
  (bind _output_get (Variables|Ref|SetTimePercent (Math|Curves|GetFloatValue (Variables|Ref|GetSunAngleCurve) _daypercent))))

(fn MainFunction
  (bind _matrix (Variables|OrbitalComponents|GetMatrix))
  (Rendering|Debug|FlushPersistentDebugLines)
  (Class|KismetSystemLibrary|FlushDebugStrings)
  (CallFunction|CalculateMyPlanet true)
  (CallFunction|CalculateMatrix)
  (CallFunction|MoveSun)
  (CallFunction|CalculateMoons)
  (if (!= (Utilities|Array|Length (Variables|OrbitalComponents|Getmoons)) (Utilities|Array|Length (Variables|OrbitalComponents|GetOtherPlanets)))
    (CallFunction|MakeMoons))
  (for (_array_element _array_index) (Variables|OrbitalComponents|Getmoons)
    (Transformation|SetWorldTransform _array_element (Math|Transform|Lerp(Transform) (Transformation|GetRelativeTransform _array_element) (Math|Transform|MakeTransform (Class|KismetMathLibrary|MatrixInverseTransformPosition _matrix (.location (Utilities|Array|Get(acopy) (Variables|OrbitalComponents|GetOtherPlanets_Dir) _array_index))) (CallFunction|InverseTransformMatrixRotation _matrix (.rotation (Utilities|Array|Get(acopy) (Variables|OrbitalComponents|GetOtherPlanets_Dir) _array_index))) (.scale (Utilities|Array|Get(acopy) (Variables|OrbitalComponents|GetOtherPlanets_Dir) _array_index))) (Utilities|Time|GetWorldDeltaSeconds)) false true))
  (CallFunction|DrawDebugDiagram))

(fn InverseTransformMatrixRotation
  (params (Matrix :type Matrix%20Structure) (Rotation :type Rotator))
  (return (Math|Rotator|MakeRotationfromAxes (Class|KismetMathLibrary|MatrixInverseTransformVector Matrix (Math|Vector|RotateVector (Math|Vector|MakeVector 1.0 0.0 0.0) Rotation)) (Class|KismetMathLibrary|MatrixInverseTransformVector Matrix (Math|Vector|RotateVector (Math|Vector|MakeVector 0.0 1.0 0.0) Rotation)) (Class|KismetMathLibrary|MatrixInverseTransformVector Matrix (Math|Vector|RotateVector (Math|Vector|MakeVector 0.0 0.0 1.0) Rotation)))))