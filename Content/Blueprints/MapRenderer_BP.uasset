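; Map renderer that takes a one-time top-down capture of the referenced Landscape when play begins.
; Derives height and altitude ranges from the landscape bounds and writes them to the MapParams material parameter collection.
; Moves MapCapture above the landscape's center, sets its ortho width to cover the larger horizontal extent, then triggers a single scene capture.
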(event EventBeginPlay
  (bind _map_capture (Variables|Default|GetMap%20Capture))
  (bind _landscape (Variables|Default|GetLandscape))
  (bind (_origin _boxextent) (Collision|GetActorBounds _landscape false false))
  (Variables|Default|SetOrigin _origin)
  (Variables|Default|SetBox%20Extent _boxextent)
  (Variables|Default|SetWorldPos (+ _origin (Math|Vector|MakeVector 0.0 0.0 (+ (.z (Variables|Default|GetBox%20Extent)) 5e+03))))
  (Rendering|Material|SetScalarParameterValue (Variables|Default|GetMapParams) (Variables|Default|GetMaxValue) (+ (.z (Variables|Default|GetOrigin)) (/ (.z (Variables|Default|GetBox%20Extent)) 2.0)) :!class /Script/Engine.KismetMaterialLibrary)
  (Rendering|Material|SetScalarParameterValue (Variables|Default|GetMapParams) (Variables|Default|GetMinValue) (- (.z (Variables|Default|GetOrigin)) (/ (.z (Variables|Default|GetBox%20Extent)) 2.0)) :!class /Script/Engine.KismetMaterialLibrary)
  (Rendering|Material|SetScalarParameterValue (Variables|Default|GetMapParams) (Variables|Default|GetMaxAlt) (+ (/ (.z (Variables|Default|GetWorldPos)) 2.0) (/ (.z (Variables|Default|GetBox%20Extent)) 2.0)) :!class /Script/Engine.KismetMaterialLibrary)
  (Rendering|Material|SetScalarParameterValue (Variables|Default|GetMapParams) (Variables|Default|GetMinAlt) (- (/ (.z (Variables|Default|GetWorldPos)) 2.0) (/ (.z (Variables|Default|GetBox%20Extent)) 2.0)) :!class /Script/Engine.KismetMaterialLibrary)
  (Transformation|SetWorldLocation _map_capture (Variables|Default|GetWorldPos) false true)
  (Variables|/Script/Engine.SceneCaptureComponent2D|SetOrthoWidth _map_capture (* (select (> (.x (Variables|Default|GetBox%20Extent)) (.y (Variables|Default|GetBox%20Extent))) (.x (Variables|Default|GetBox%20Extent)) (.y (Variables|Default|GetBox%20Extent))) 2.0))
  (Rendering|SceneCapture|CaptureScene _map_capture :!class /Script/Engine.SceneCaptureComponent2D))

(fn ConstructionScript)