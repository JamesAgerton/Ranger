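; Tactical camera pawn that starts at the player character's location, with its spring arm at a set pitch and the controller's yaw.
; Movement input follows control yaw on the horizontal plane, with axis scaling that compensates for gamepad diagonals.
; Each tick, a vertical sphere trace on the Camera channel snaps its height to the surface, ignoring actors tagged IgnoreMe.
; Character-state interface getters return placeholder defaults.
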(event Custom|Start
  (Transformation|SetWorldRotation (Variables|Default|GetSpringArm) (Math|Rotator|MakeRotator 0.0 (Variables|Default|GetTacticalCamPitch) (.yaw (Pawn|GetControlRotation (Game|GetPlayerController 0) :!class /Script/Engine.Controller))) false false)
  (Transformation|SetWorldLocation (Variables|Default|GetScene) (Transformation|GetActorLocation (Variables|Default|GetMainCharacter)) false false))

(event EventBeginPlay
  (Variables|Default|SetMainCharacter (Game|GetPlayerCharacter 0))
  (bind _outactors (Actor|GetAllActorswithTag "IgnoreMe"))
  (Variables|Default|SetIgnored _outactors))

(event EventBPIInputMovement
  (params (ForwardAxis :type Boolean))
  (bind _returnvalue (Pawn|GetControlRotation :!class /Script/Engine.Pawn))
  (bind _returnvalue_2 (Input|AxisValues|GetForward))
  (bind _returnvalue_3 (Input|AxisValues|GetRight))
  (bind (_y_out _x_out) (Input|FixDiagonalGamepadValues _returnvalue_2 _returnvalue_3))
  (if ForwardAxis
    (Pawn|Input|AddMovementInput (Math|Vector|GetForwardVector (Math|Rotator|MakeRotator 0.0 0.0 (.yaw _returnvalue))) _y_out false)
    (else
      (Pawn|Input|AddMovementInput (Math|Vector|GetRightVector (Math|Rotator|MakeRotator 0.0 0.0 (.yaw _returnvalue))) _x_out false))))

(event EventTick
  (params (DeltaSeconds :type Float%20%28single-precision%29))
  (CallFunction|CorrectHoverHeight))

(fn ConstructionScript)

(fn FixDiagonalGamepadValues
  (params (Y%20in :type Float%20%28double-precision%29) (X%20in :type Float%20%28double-precision%29))
  (return (Math|Float|Clamp(Float) (* Y%20in (Math|Float|MapRangeClamped (Math|Float|Absolute(Float) X%20in) 0.0 0.6 1.0 1.2)) -1.0) (Math|Float|Clamp(Float) (* X%20in (Math|Float|MapRangeClamped (Math|Float|Absolute(Float) Y%20in) 0.0 0.6 1.0 1.2)) -1.0)))

(fn CorrectHoverHeight
  (bind _returnvalue (Transformation|GetActorLocation))
  (bind _showdebugshapes (Class|RCharacterBPI|BPIGetDebugInfo(Message) (Game|GetPlayerController 0)))
  (bind (_outhit _returnvalue_2) (Collision|SphereTraceByChannel (+ _returnvalue "0.000000,0,600.000000") (- _returnvalue "0,0,600.000000") 5e+01 "TraceTypeQuery2" false (Variables|Default|GetIgnored) (select _showdebugshapes "ForOneFrame" "None")))
  (if _returnvalue_2
    (if (> (Math|Float|Absolute(Float) (.z (- (.Location (Collision|BreakHitResult _outhit)) (Transformation|GetActorLocation)))) 0.1)
      (Transformation|AddActorWorldOffset (Math|Vector|MakeVector 0.0 0.0 (.z (- (.Location (Collision|BreakHitResult _outhit)) (Transformation|GetActorLocation))))))))

(fn BPIGetCameraMode
  (return "NewEnumerator0"))

(fn BPIGetCurrentStates
  (return "MOVE_None" "NewEnumerator0" "NewEnumerator0" "NewEnumerator0" "NewEnumerator0" "NewEnumerator0" "NewEnumerator0"))

(fn BPIGetDebugInfo
  (return 0 false))

(fn BPIGetEssentialValues
  (return "0, 0, 0" "0, 0, 0" "0, 0, 0" false false 0.0 0.0 "0, 0, 0" 0.0))