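; Monster gallery actor that spawns several randomized examples of every species in R_SpeciesEncyclopedia_Table, laid out in a grid.
; ScaleCalc sizes the floor from species count, example count and separation, and LocationCalc builds the grid points.
; BeginPlay line-traces at each point to place an R_Base_Monster_BP, then calls SERVERRandomMonster on it.
; Debug drawing previews bounds and points from the Construction Script and on every Tick.
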(event EventBeginPlay
  (bind _exampleamount (Variables|Default|GetExampleAmount))
  (Utilities|FlowControl|Sequence
    (:then_0
      (bind _outrownames (DataTable|GetDataTableRowNames "/Game/Blueprints/Monsters/DataStructures/Tables/R_SpeciesEncyclopedia_Table.R_SpeciesEncyclopedia_Table"))
      (Variables|Default|SetOut%20Row%20Names _outrownames)
      (Variables|Default|SetSpeciesCount (Utilities|Array|Length _outrownames)))
    (:then_1
      (CallFunction|ScaleCalc)
      (Transformation|SetWorldScale3D (Variables|Default|GetFloor) (Math|Vector|MakeVector (Variables|Default|GetScaleX) (Variables|Default|GetScaleY) 1.0))
      (CallFunction|LocationCalc))
    (:then_2
      (for _index (range 0 (- (Variables|Default|GetSpeciesCount) 1))
        (for _index_2 (range 0 (- _exampleamount 1))
          (bind _outhit (Collision|LineTraceByChannel (+ (Utilities|Array|Get(acopy) (Variables|Default|GetLocations) (+ _index_2 (* _index _exampleamount))) "0, 0,100.000000") (+ (Utilities|Array|Get(acopy) (Variables|Default|GetLocations) (+ _index_2 (* _index _exampleamount))) "0, 0,-100.000000") "TraceTypeQuery1" false 0 "None"))
          (bind _returnvalue (Game|SpawnActorfromClass :Class "/Game/Blueprints/Monsters/R_Base_Monster_BP.R_Base_Monster_BP_C" :SpawnTransform (Math|Transform|MakeTransform (.Location (Collision|BreakHitResult _outhit)) "0,90.000000, 0" "1,1,1") :CollisionHandlingOverride "AlwaysSpawn" :SpeciesIndex (Utilities|Array|Get(acopy) (Variables|Default|GetOut%20Row%20Names) _index) :Instigator 0))
          (Default|SERVERRandomMonster _returnvalue))))))

(event EventTick
  (params (DeltaSeconds :type Float%20%28single-precision%29))
  (CallFunction|DrawDebug))

(fn ConstructionScript
  (Utilities|FlowControl|Sequence
    (:then_0
      (bind _outrownames (DataTable|GetDataTableRowNames "/Game/Blueprints/Monsters/DataStructures/Tables/R_SpeciesEncyclopedia_Table.R_SpeciesEncyclopedia_Table"))
      (Variables|Default|SetSpeciesCount (Utilities|Array|Length _outrownames))
      (CallFunction|ScaleCalc)
      (CallFunction|LocationCalc))
    (:then_1
      (CallFunction|DrawDebug))))

(fn ScaleCalc
  (bind _floor (Variables|Default|GetFloor))
  (bind _min (Components|StaticMesh|GetLocalBounds _floor))
  (Variables|Default|SetScaleX (/ (* (+ (Variables|Default|GetSpeciesCount) 1) (Variables|Default|GetSeperation)) (.x _min)))
  (Variables|Default|SetScaleY (/ (* (+ (Variables|Default|GetExampleAmount) 1) (Variables|Default|GetSeperation)) (.y _min)))
  (Variables|Default|SetExtentX (* (.x _min) (Variables|Default|GetScaleX)))
  (Variables|Default|SetExtentY (* (.y _min) (Variables|Default|GetScaleY))))

(fn LocationCalc
  (Utilities|FlowControl|Sequence
    (:then_0
      (Utilities|Array|Clear (Variables|Default|GetLocations)))
    (:then_1
      (for _index (range 1 (Variables|Default|GetSpeciesCount))
        (LocalVariables|SetSpeciesIndex _index)
        (for _index_2 (range 1 (Variables|Default|GetExampleAmount))
          (LocalVariables|SetExampleIndex _index_2)
          (bind _output_get (LocalVariables|SetPos (Math|Vector|MakeVector (+ (* (Variables|Default|GetExtentX) -1.0) (* (LocalVariables|GetSpeciesIndex) (* (Variables|Default|GetSeperation) (select (== (LocalVariables|GetSpeciesIndex) 1) 2.0 2.0)))) (+ (* (Variables|Default|GetExtentY) -1.0) (* (LocalVariables|GetExampleIndex) (* (Variables|Default|GetSeperation) (select (== (LocalVariables|GetExampleIndex) 1) 2.0 2.0)))) 5e+01)))
          (Utilities|Array|Add (Variables|Default|GetLocations) (+ _output_get (Transformation|GetWorldLocation (Variables|Default|GetFloor)))))))))

(fn DrawDebug
  (Rendering|Debug|FlushPersistentDebugLines)
  (Rendering|Debug|DrawDebugBox (Transformation|GetWorldLocation (Variables|Default|GetFloor)) (* (Math|Vector|MakeVector (Variables|Default|GetScaleX) (Variables|Default|GetScaleY) 1.0) (.Min (Components|StaticMesh|GetLocalBounds (Variables|Default|GetFloor)))) "(R=0.000000,G=0.875069,B=1.000000,A=1.000000)" "0, 0, 0" (Variables|Default|GetDebugDrawTime) 3.0)
  (for _array_element (Variables|Default|GetLocations)
    (Rendering|Debug|DrawDebugPoint _array_element 3.0 "(R=1.000000,G=1.000000,B=1.000000,A=1.000000)" (Variables|Default|GetDebugDrawTime))))