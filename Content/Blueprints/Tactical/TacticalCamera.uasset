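; Tactical camera pawn that starts over the player character, pans by movement input and shows a ground target decal.
; Each tick a sphere trace corrects its height, while the decal follows the cursor or recenters for gamepad use.
; In combat, AutoPath runs a navigation query between the decal and a given location, feeding a spline along which pooled decal actors are placed to draw the path.
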(event Custom|Start
  (Transformation|SetWorldRotation (Variables|Default|GetSpringArm) (Math|Rotator|MakeRotator 0.0 (Variables|Default|GetTacticalCamPitch) (.yaw (Pawn|GetControlRotation (Game|GetPlayerController 0) :!class /Script/Engine.Controller))) false false)
  (Transformation|SetWorldLocation (Variables|Default|GetScene) (Transformation|GetActorLocation (Variables|Default|GetMainCharacter)) false false)
  (CallFunction|TurnonTarget))

(event Custom|ResetTargetLocation
  (bind _targetdecal (Variables|Default|GetTargetDecal))
  (if (> (Math|Vector|Distance(Vector) (Variables|/Script/Engine.SceneComponent|GetRelativeLocation _targetdecal) "0, 0, 0") 0.01)
    (Transformation|SetRelativeLocation _targetdecal "0, 0, 0" false false)))

(event Custom|TurnOnTarget
  (Rendering|SetVisibility (Variables|Default|GetTargetDecal) true false))

(event Custom|TurnOffTarget
  (Rendering|SetVisibility (Variables|Default|GetTargetDecal) false false))

(event Custom|Stop
  (CallFunction|TurnOffTarget)
  (CallFunction|HidePath))

(event Custom|Show%20Path
  (params (TargetLocation :type Vector))
  (bind _targetdecal (Variables|Default|GetTargetDecal))
  (bind _spline (Variables|Default|GetSpline))
  (bind _pathdecalseperation (Variables|Default|GetPathDecalSeperation))
  (bind _returnvalue (Transformation|GetWorldLocation _targetdecal))
  ;[1 1 1] Draw the path on the ground
  (Utilities|FlowControl|Sequence
    (:then_0
      (bind _outhit (Collision|LineTraceByChannel (+ _returnvalue "0,0,80.000000") (- _returnvalue "0,0,80.000000") "TraceTypeQuery1" false 0 "None"))
      (bind _returnvalue_2 (Class|NavigationSystemV1|FindPathtoLocationSynchronously (.Location (Collision|BreakHitResult _outhit)) TargetLocation 0 0))
      (Spline|ClearSplinePoints (Variables|Default|GetSpline) true)
      (for _array_element (Variables|/Script/NavigationSystem.NavigationPath|GetPathPoints _returnvalue_2)
        (Spline|AddSplinePoint (Variables|Default|GetSpline) _array_element "World" true)))
    (:then_1
      (for _array_element_2 (Variables|Default|GetPathDecalPool)
        (Rendering|SetVisibility (Variables|/Game/Blueprints/Tactical/PathDecalActor_BP.PathDecalActor_BP_C|GetPathDecal _array_element_2) false false))
      (for _index (range 1 (Math|Float|Truncate (Math|Float|%(Float) (Spline|GetSplineLength _spline) _pathdecalseperation)))
        (Utilities|IsValid (Utilities|Array|Get(acopy) (Variables|Default|GetPathDecalPool) _index)
          (:Is%20Valid
            (Transformation|SetActorLocation (Utilities|Array|Get(acopy) (Variables|Default|GetPathDecalPool) _index) (Spline|GetLocationatDistanceAlongSpline _spline (* _pathdecalseperation _index) "World") false false)
            (Rendering|SetVisibility (Variables|/Game/Blueprints/Tactical/PathDecalActor_BP.PathDecalActor_BP_C|GetPathDecal (Utilities|Array|Get(acopy) (Variables|Default|GetPathDecalPool) _index)) true false))
          (:Is%20Not%20Valid
            (bind _returnvalue_3 (Game|SpawnActorfromClass "/Game/Blueprints/Tactical/PathDecalActor_BP.PathDecalActor_BP_C" (Math|Transform|MakeTransform (Spline|GetLocationatDistanceAlongSpline _spline (* _pathdecalseperation _index) "World") "0, 0, 0" "1.000000,1.000000,1.000000") "Undefined" self 0))
            (Utilities|Array|Add (Variables|Default|GetPathDecalPool) _returnvalue_3)
            (Rendering|SetVisibility (Variables|/Game/Blueprints/Tactical/PathDecalActor_BP.PathDecalActor_BP_C|GetPathDecal _returnvalue_3) true false)))))))

(event Custom|HidePath
  (for _array_element (Variables|Default|GetPathDecalPool)
    (Rendering|SetVisibility (Variables|/Game/Blueprints/Tactical/PathDecalActor_BP.PathDecalActor_BP_C|GetPathDecal _array_element) false false)))

(event Custom|AutoPath
  (params (Show :type Boolean) (ActorLocation :type Vector))
  (bind _astest_game_mode_gm (Utilities|Casting|CastToTestGameMode_GM (Game|GetGameMode)))
  (if (and (Variables|/Game/Blueprints/Core/TestGameMode_GM.TestGameMode_GM_C|GetInCombat _astest_game_mode_gm) Show)
    (CallFunction|ShowPath ActorLocation)
    (else
      (CallFunction|HidePath))))

(event EventBeginPlay
  (Variables|Default|SetMainCharacter (Game|GetPlayerCharacter 0))
  (bind _outactors (Actor|GetAllActorswithTag "IgnoreMe"))
  (Variables|Default|SetIgnored _outactors))

(event EventBPIInputMovement
  (params (ForwardAxis :type Boolean))
  (bind _returnvalue (Pawn|GetControlRotation :!class /Script/Engine.Pawn))
  (bind _returnvalue_2 (Input|AxisValues|GetForward))
  (bind _returnvalue_3 (Input|AxisValues|GetRight))
  (bind (_y_out _x_out) (Input|FixDiagonalGamepadValues _returnvalue_2 _returnvalue_3))
  (if ForwardAxis
    (Pawn|Input|AddMovementInput (Math|Vector|GetForwardVector (Math|Rotator|MakeRotator 0.0 0.0 (.yaw _returnvalue))) _y_out false)
    (else
      (Pawn|Input|AddMovementInput (Math|Vector|GetRightVector (Math|Rotator|MakeRotator 0.0 0.0 (.yaw _returnvalue))) _x_out false))))

(event EventTick
  (params (DeltaSeconds :type Float%20%28single-precision%29))
  (CallFunction|CorrectHoverHeight)
  (bind _usinggamepad (Class|RCharacterBPI|BPIGetDebugInfo(Message) (Game|GetPlayerController 0)))
  (if _usinggamepad
    (Utilities|FlowControl|DoOnce false :!label _label
      (:Completed
        (CallFunction|ResetTargetLocation)))
    (else
      (CallFunction|TargetFollowCursor)
      (goto _label Reset))))

(fn ConstructionScript)

(fn FixDiagonalGamepadValues
  (params (Y%20in :type Float%20%28double-precision%29) (X%20in :type Float%20%28double-precision%29))
  (return (Math|Float|Clamp(Float) (* Y%20in (Math|Float|MapRangeClamped (Math|Float|Absolute(Float) X%20in) 0.0 0.6 1.0 1.2)) -1.0) (Math|Float|Clamp(Float) (* X%20in (Math|Float|MapRangeClamped (Math|Float|Absolute(Float) Y%20in) 0.0 0.6 1.0 1.2)) -1.0)))

(fn CorrectHoverHeight
  (bind _returnvalue (Transformation|GetActorLocation))
  (bind _showdebugshapes (Class|RCharacterBPI|BPIGetDebugInfo(Message) (Game|GetPlayerController 0)))
  (bind (_outhit _returnvalue_2) (Collision|SphereTraceByChannel (+ _returnvalue "0.000000,0,600.000000") (- _returnvalue "0,0,600.000000") 5e+01 "TraceTypeQuery2" false (Variables|Default|GetIgnored) (select _showdebugshapes "ForOneFrame" "None")))
  (if _returnvalue_2
    (if (> (Math|Float|Absolute(Float) (.z (- (.Location (Collision|BreakHitResult _outhit)) (Transformation|GetActorLocation)))) 0.1)
      (Transformation|AddActorWorldOffset (Math|Vector|MakeVector 0.0 0.0 (.z (- (.Location (Collision|BreakHitResult _outhit)) (Transformation|GetActorLocation))))))))

(fn TargetFollowCursor
  (Transformation|SetWorldLocation (Variables|Default|GetTargetDecal) (.Location (Collision|BreakHitResult (.HitResult (Game|Player|GetHitResultUnderCursorbyChannel (Game|GetPlayerController 0) "TraceTypeQuery2" true)))) false false))

(fn BPIGetCameraMode
  (return "NewEnumerator0"))

(fn BPIGetCurrentStates
  (return "MOVE_None" "NewEnumerator0" "NewEnumerator0" "NewEnumerator0" "NewEnumerator0" "NewEnumerator0" "NewEnumerator0"))

(fn BPIGetDebugInfo
  (return 0 false false))

(fn BPIGetEssentialValues
  (return "0, 0, 0" "0, 0, 0" "0, 0, 0" false false 0.0 0.0 "0, 0, 0" 0.0))