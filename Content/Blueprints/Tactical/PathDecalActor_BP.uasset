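; Tactical path marker actor that shows a decal tinted by whether the path is active or inactive.
; On BeginPlay it creates a dynamic material instance from the decal's material and sets its Color parameter to the active color.
; PathDecalActivate and PathDecalDeactivate switch that Color parameter between the active and inactive colors.
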(event EventBeginPlay
  (bind _returnvalue (Rendering|Material|CreateDynamicMaterialInstance (Class|DecalComponent|GetDecalMaterial (Variables|Default|GetPathDecal)) "None" "None" :!class /Script/Engine.KismetMaterialLibrary))
  (bind _output_get (Variables|Default|SetDecalMaterial _returnvalue))
  (Rendering|Material|SetVectorParameterValue _output_get "Color" (Variables|Default|GetActiveColor) :!class /Script/Engine.MaterialInstanceDynamic))

(fn ConstructionScript)

(fn PathDecalActivate
  (Rendering|Material|SetVectorParameterValue (Variables|Default|GetDecalMaterial) "Color" (Variables|Default|GetActiveColor) :!class /Script/Engine.MaterialInstanceDynamic))

(fn PathDecalDeactivate
  (Rendering|Material|SetVectorParameterValue (Variables|Default|GetDecalMaterial) "Color" (Variables|Default|GetInactiveColor) :!class /Script/Engine.MaterialInstanceDynamic))