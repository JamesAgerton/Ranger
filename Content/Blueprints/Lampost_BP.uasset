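; Lamp post actor that switches its spotlight on at sunset and off at sunrise.
; On BeginPlay it casts the game state to R_GS_Framework and binds handlers to its sunset and sunrise events.
; The handlers set the spotlight intensity to a configurable value or to zero.
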(event Custom|TurnOn
  (Rendering|Components|Light|SetIntensity (Variables|Default|GetSpotLight) (Variables|Default|GetNew%20Intensity)))

(event Custom|TurnOff
  (Rendering|Components|Light|SetIntensity (Variables|Default|GetSpotLight) 0.0))

(event EventBeginPlay
  (bind _asr_gs_framework (Utilities|Casting|CastToR_GS_Framework (Game|GetGameState)))
  (Variables|Default|SetGameStateRef _asr_gs_framework)
  (EventDispatchers|BindEventtoSunset (Variables|Default|GetGameStateRef) (delegate Custom|TurnOn))
  (EventDispatchers|BindEventtoSunrise (Variables|Default|GetGameStateRef) (delegate Custom|TurnOff)))

(fn ConstructionScript)